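; BP_Point is a capture point Blueprint that raises a flag while an actor overlaps it.
; Overlap begin plays or restarts a timeline whose FlagUp track sets Value and flag height, unless Value already reaches the owned threshold.
; Overlap end reverses the timeline at half rate unless Value equals one, and the Capturing boolean tracks overlap.
; Any actor triggers capture, with debug prints reporting progress or ownership.
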(event `self.ReceiveActorBeginOverlap`
  (params (OtherActor :type "Actor Object Reference"))
  (`parent.ReceiveActorBeginOverlap` OtherActor)
  (set `self.capturing` true)
  (if (>= (`self.value`) 10.0)
    (`KismetSystemLibrary.PrintString` "c'est déja votre point !")
    (elif (!= (`self.value`) 0.0)
      (bind (_direction _flag_up) (`Timeline|Timeline` :!label _label)
        (:`Update`
          (switch `ETimelineDirection` _direction
            (:`Forward`
              (`TimelineComponent.SetPlayRate` (`self.Timeline`) 1.0)
              (bind _output_get (set `self.value` _flag_up)))
            (:`Backward`
              (`TimelineComponent.SetPlayRate` (`self.Timeline`) 0.5)
              (set `self.value` _flag_up)))
          (`SceneComponent.K2_SetRelativeLocation` (`self.flag`) (`KismetMathLibrary.MakeVector` 0.0 0.0 (* _output_get 700.0)) false false)
          (`KismetSystemLibrary.PrintString` (`KismetStringLibrary.Conv_DoubleToString` (`self.value`)))))
      (else
        (goto _label :!via `PlayFromStart`)))))

(event `self.ReceiveActorEndOverlap`
  (params (OtherActor :type "Actor Object Reference"))
  (set `self.capturing` false)
  (if (not (== (`self.value`) 1.0))
    (goto _label :!via `Reverse`)))

(fn `UserConstructionScript`
  (`parent.UserConstructionScript`))