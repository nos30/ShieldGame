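; Stick switch interactable that releases the drawbridge when the player interacts with it.
; InteractAction calls ReleaseDoor on the BP_D_Drawbridge found through GetActorOfClass and plays a timeline that pitches the stick toward MaxSwitchAngle at StickSwitchMovingSpeed.
; Ending overlap with the collision sphere, gated by a main character cast, reverses the timeline without calling the drawbridge.
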(event `OpenDoor`
  (bind _returnvalue (`GameplayStatics.GetActorOfClass` "/Game/ShieldGame/Blueprints/Objects/Decors_Objects/Doors/DrawBridge/BP_D_Drawbridge.BP_D_Drawbridge_C"))
  (`/Game/ShieldGame/Blueprints/Objects/Decors_Objects/Doors/DrawBridge/RI_D_Drawbridge.ReleaseDoor` _returnvalue)
  (bind (_direction _newtrack_0) (`Timeline|Timeline` :!label _label)
    (:`Update`
      (switch `ETimelineDirection` _direction
        (:`Forward`
          _)
        (:`Backward`
          _))
      (`TimelineComponent.SetPlayRate` (`self.Timeline`) (`self.StickSwitchMovingSpeed`))
      (`SceneComponent.K2_SetRelativeRotation` (`self.StickSwitch`) (`KismetMathLibrary.MakeRotator` 0.0 (* _newtrack_0 (`self.MaxSwitchAngle`))) false false))))

(event `CloseDoor`
  (goto _label :!via `Reverse`))

(event `/Game/ShieldGame/Blueprints/Characters/RI_InteractAction.InteractAction`
  (`self.OpenDoor`))

(event `self.collision sphere.OnComponentEndOverlap`
  (params (OverlappedComponent :type "PrimitiveComponent Object Reference") (OtherActor :type "Actor Object Reference") (OtherComp :type "PrimitiveComponent Object Reference") (OtherBodyIndex :type Integer))
  (castclass `/Game/ShieldGame/Blueprints/Characters/BP_MainCharacter_GameMode` "/Game/ShieldGame/Blueprints/Characters/BP_MainCharacter_GameMode.BP_MainCharacter_GameMode_C")
  (`self.CloseDoor`))

(fn `UserConstructionScript`
  (`parent.UserConstructionScript`))