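; BP_AO_Campfire is an interactable campfire whose fire can be toggled on and off.
; A collision sphere sets a flag while any actor overlaps it and clears it when an overlap ends.
; When that flag is set, InteractAction runs a FlipFlop that alternately shows and hides the FireLight and NGFire components, starting with show.
; The construction script only calls its parent's.
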(event `/Game/ShieldGame/Blueprints/Characters/RI_InteractAction.InteractAction`
  (if (`self.IsOnCollisionSphere`)
    (`/Engine/EditorBlueprintResources/StandardMacros.FlipFlop`
      (:`A`
        (`SceneComponent.SetVisibility` (`self.FireLight`) true false)
        (`SceneComponent.SetVisibility` (`self.NG_Fire`) true false))
      (:`B`
        (`SceneComponent.SetVisibility` (`self.FireLight`) false false)
        (`SceneComponent.SetVisibility` (`self.NG_Fire`) false false)))))

(event `self.collision sphere.OnComponentBeginOverlap`
  (params (OverlappedComponent :type "PrimitiveComponent Object Reference") (OtherActor :type "Actor Object Reference") (OtherComp :type "PrimitiveComponent Object Reference") (OtherBodyIndex :type Integer) (bFromSweep :type Boolean) (SweepResult :type "HitResult Structure (by ref)"))
  (set `self.IsOnCollisionSphere` true))

(event `self.collision sphere.OnComponentEndOverlap`
  (params (OverlappedComponent :type "PrimitiveComponent Object Reference") (OtherActor :type "Actor Object Reference") (OtherComp :type "PrimitiveComponent Object Reference") (OtherBodyIndex :type Integer))
  (set `self.IsOnCollisionSphere` false))

(fn `UserConstructionScript`
  (`parent.UserConstructionScript`))