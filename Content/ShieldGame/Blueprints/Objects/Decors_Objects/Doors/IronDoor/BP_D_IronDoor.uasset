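; BP_D_IronDoor is an iron door whose grille slides open automatically when BP_MainCharacter_GameMode enters its collision sphere and closes when it leaves.
; Overlap begin and end events, filtered by that cast, call OpenDoor and CloseDoor to play or reverse a shared timeline.
; Each timeline update applies DoorOpenningSpeed as play rate and moves the grille's relative Z by the track value scaled by MaxOpenningDoorLocation.
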(event `OpenDoor`
  (bind (_direction _newtrack_0) (`Timeline|Timeline` :!label _label)
    (:`Update`
      (switch `ETimelineDirection` _direction
        (:`Forward`
          _)
        (:`Backward`
          _))
      (`TimelineComponent.SetPlayRate` (`self.Timeline`) (`self.DoorOpenningSpeed`))
      (`SceneComponent.K2_SetRelativeLocation` (`self.Grille`) (`KismetMathLibrary.MakeVector` 0.0 0.0 (* _newtrack_0 (`self.MaxOpenningDoorLocation `))) false false))))

(event `CloseDoor`
  (goto _label :!via `Reverse`))

(event `self.collision sphere.OnComponentBeginOverlap`
  (params (OverlappedComponent :type "PrimitiveComponent Object Reference") (OtherActor :type "Actor Object Reference") (OtherComp :type "PrimitiveComponent Object Reference") (OtherBodyIndex :type Integer) (bFromSweep :type Boolean) (SweepResult :type "HitResult Structure (by ref)"))
  (castclass `/Game/ShieldGame/Blueprints/Characters/BP_MainCharacter_GameMode` "/Game/ShieldGame/Blueprints/Characters/BP_MainCharacter_GameMode.BP_MainCharacter_GameMode_C")
  (`self.OpenDoor`))

(event `self.collision sphere.OnComponentEndOverlap`
  (params (OverlappedComponent :type "PrimitiveComponent Object Reference") (OtherActor :type "Actor Object Reference") (OtherComp :type "PrimitiveComponent Object Reference") (OtherBodyIndex :type Integer))
  (castclass `/Game/ShieldGame/Blueprints/Characters/BP_MainCharacter_GameMode` "/Game/ShieldGame/Blueprints/Characters/BP_MainCharacter_GameMode.BP_MainCharacter_GameMode_C")
  (`self.CloseDoor`))

(fn `UserConstructionScript`
  (`parent.UserConstructionScript`))