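; Throwable spear actor, a work in progress, meant to stick into whatever it hits.
; When the spear component hits something other than player pawn 0, it stops projectile movement, snaps to the impact point and disables gravity.
; It also tries to attach the actor to ElementHit, but the assignment of that variable from the hit component is disconnected.
; Other physics and collision-disabling experiments are left unwired.
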(event `self.Spear.OnComponentWake`
  (params (WakingComponent :type "PrimitiveComponent Object Reference") (BoneName :type Name)))

(event `self.Capsule.OnComponentHit`
  (params (HitComponent :type "PrimitiveComponent Object Reference") (OtherActor :type "Actor Object Reference") (OtherComp :type "PrimitiveComponent Object Reference") (NormalImpulse :type "Vector Structure") (Hit :type "HitResult Structure (by ref)")))

(event `self.Spear.OnComponentHit`
  (params (HitComponent :type "PrimitiveComponent Object Reference") (OtherActor :type "Actor Object Reference") (OtherComp :type "PrimitiveComponent Object Reference") (NormalImpulse :type "Vector Structure") (Hit :type "HitResult Structure (by ref)"))
  ;[1 1 1] HitSpear dev
  (if (and (!= HitComponent self) (!= OtherActor (`GameplayStatics.GetPlayerPawn` 0)))
    (`MovementComponent.StopMovementImmediately` (`self.ProjectileMovement`))
    (`SceneComponent.K2_SetWorldLocation` (`self.Spear`) Hit_ImpactPoint false false)
    ;[1 1 1] non terminé attacher la spear dès la colision
    (`self.K2_AttachToComponent` (`ActorComponent.GetOwner` (`self.Spear`)) (`self.ElementHit`) "None" "SnapToTarget" "SnapToTarget" "SnapToTarget" false)
    (`PrimitiveComponent.SetEnableGravity` (`self.Spear`) false)))

(fn `UserConstructionScript`)